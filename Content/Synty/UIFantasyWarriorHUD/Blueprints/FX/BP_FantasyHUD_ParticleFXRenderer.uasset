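; Actor that renders Niagara particle effects through a scene capture for the Fantasy Warrior HUD.
; On begin play, its SceneCaptureComponent2D uses a show-only list containing this actor and its children.
; SpawnParticleSystems destroys earlier systems, spawns the requested ones at the actor's transform and registers each with the capture.
; External callers, such as the VFX sample page, toggle per-frame capture through StartCapture and StopCapture for efficiency.
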(event Custom|SpawnParticleSystems
  (params (NiagaraSystems :type Array%20of%20Niagara%20System%20Object%20References))
  ;[1 1 1] Spawn Particle Systems - deletes any currently active particles used by this system, then spawns the desired ones, and adds them to the scene capture
  (bind _arrayelement (Utilities|Array|ReverseforEachLoop (Variables|Default|GetActiveNiagaraSystems))
    (:LoopBody
      (Utilities|IsValid _arrayelement
        (:Is%20Valid
          (Components|DestroyComponent _arrayelement))))
    (:Completed
      (for _array_element NiagaraSystems
        (bind _returnvalue (Niagara|SpawnSystematLocation _array_element (Transformation|GetActorLocation) (Transformation|GetActorRotation)))
        (Utilities|Array|Add (Variables|Default|GetActiveNiagaraSystems) _returnvalue)
        (Rendering|SceneCapture|ShowOnlyComponent (Variables|Default|GetSceneCaptureComponent2D) _returnvalue)))))

(event Custom|StartCapture
  ;[1 1 1] Start/Stop capture
  ; Enables/Disables Capture Every Frame
  ; Called externally (by the VFX sample page, for example) when particles are spawned/disabled for efficiency
  (Variables|/Script/Engine.SceneCaptureComponent|SetbCaptureEveryFrame (Variables|Default|GetSceneCaptureComponent2D) true))

(event Custom|StopCapture
  ;[1 1 1] Start/Stop capture
  ; Enables/Disables Capture Every Frame
  ; Called externally (by the VFX sample page, for example) when particles are spawned/disabled for efficiency
  (Variables|/Script/Engine.SceneCaptureComponent|SetbCaptureEveryFrame (Variables|Default|GetSceneCaptureComponent2D) false))

(event EventBeginPlay
  ;[1 1 1] Begin play - Tell the scene capture component to only capture this actor and it's children
  (Rendering|SceneCapture|ShowOnlyActorComponents (Variables|Default|GetSceneCaptureComponent2D) self true))

(fn ConstructionScript)