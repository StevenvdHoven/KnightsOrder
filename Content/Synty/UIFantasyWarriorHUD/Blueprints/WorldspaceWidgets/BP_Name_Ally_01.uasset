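; BP_Name_Ally_01 is a world-space nameplate actor from the Synty Fantasy Warrior HUD pack, named for labeling allies.
; Its construction script passes a non-empty DisplayText to the Widget component's HUD_FantasyWarrior_NameBase_01 through UpdateWidget.
; The event graph holds only disabled default events, so the actor's own graphs add no runtime logic.
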(event EventBeginPlay
  (|CallParentFunction) ; This node is disabled and will not be called.\nDrag off pins to build functionality.
)

(event Collision|EventActorBeginOverlap
  (params (OtherActor :type Actor%20Object%20Reference))
  (|CallParentFunction OtherActor) ; This node is disabled and will not be called.\nDrag off pins to build functionality.
)

(event EventTick
  (params (DeltaSeconds :type Float%20%28single-precision%29))
  (|CallParentFunction DeltaSeconds) ; This node is disabled and will not be called.\nDrag off pins to build functionality.
)

(fn ConstructionScript
  (|CallParentFunction)
  (if (not (Utilities|Text|TextIsEmpty (Variables|Synty|GetDisplayText)))
    (bind _ashud_fantasy_warrior_name_base_01 (Utilities|Casting|CastToHUD_FantasyWarrior_NameBase_01 (UserInterface|GetWidget (Variables|Default|GetWidget))))
    (Default|UpdateWidget _ashud_fantasy_warrior_name_base_01 (Variables|Synty|GetDisplayText))))