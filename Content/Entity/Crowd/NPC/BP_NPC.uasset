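; BP_NPC is an always-interactable crowd NPC that gives the player a short dialogue exchange.
; On BeginPlay it picks a random Nomad body mesh and a random hair mesh for variety.
; Interact calls TalkToNPC, has the player controller present a dialogue camera centered between both actors, and shows a dialogue widget with a random available line.
; Clicking the widget removes it and turns off the dialogue camera.
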(event Custom|OnClicked_Event
  (Widget|RemovefromParent (stale EventInteract _returnvalue_2))
  (bind _asbp_player_controller (Utilities|Casting|CastToBP_PlayerController (Game|GetPlayerController 0)))
  (Default|PresentDialogueCamera _asbp_player_controller false "0, 0, 0" "0, 0, 0"))

(event EventBeginPlay
  (Components|SkeletalMesh|SetSkeletalMeshAsset (Variables|Character|GetMesh) (.OutItem (Utilities|Array|Random (Utilities|Array|MakeArray "/Game/Synty/PolygonDungeonRealms/Meshes/CharactersUE4Mannequin/SK_Chr_Nomad_Male_01.SK_Chr_Nomad_Male_01" "/Game/Synty/PolygonDungeonRealms/Meshes/CharactersUE4Mannequin/SK_Chr_Nomad_Male_02.SK_Chr_Nomad_Male_02" "/Game/Synty/PolygonDungeonRealms/Meshes/CharactersUE4Mannequin/SK_Chr_Nomad_Male_03.SK_Chr_Nomad_Male_03" "/Game/Synty/PolygonDungeonRealms/Meshes/CharactersUE4Mannequin/SK_Chr_Nomad_Female_01.SK_Chr_Nomad_Female_01" "/Game/Synty/PolygonDungeonRealms/Meshes/CharactersUE4Mannequin/SK_Chr_Nomad_Female_02.SK_Chr_Nomad_Female_02"))))
  (Components|StaticMesh|SetStaticMesh (Variables|Default|GetHeadWear) (.OutItem (Utilities|Array|Random (Utilities|Array|MakeArray "/Game/Synty/PolygonDungeonRealms/Meshes/CharacterAttachments/SM_Chr_Attach_Hair_Hero_Female_01.SM_Chr_Attach_Hair_Hero_Female_01" "/Game/Synty/PolygonDungeonRealms/Meshes/CharacterAttachments/SM_Chr_Attach_Hair_Hero_Male_01.SM_Chr_Attach_Hair_Hero_Male_01" "/Game/Synty/PolygonDungeonRealms/Meshes/CharacterAttachments/SM_Chr_Attach_Hair_Wild_01.SM_Chr_Attach_Hair_Wild_01")))))

(event EventInteract
  (params (InteractingActor :type Actor%20Object%20Reference))
  (bind (_outspeakername _outavailabledialogues) (Class|NPCCharacter|GetDialogueInfo))
  (bind _returnvalue (Transformation|GetActorLocation))
  (Utilities|FlowControl|Sequence
    (:then_0
      (Class|NPCCharacter|TalktoNPC (Transformation|GetActorLocation InteractingActor) InteractingActor)
      (bind _asbp_player (Utilities|Casting|CastToBP_Player InteractingActor))
      (bind _asbp_player_controller (Utilities|Casting|CastToBP_PlayerController (Pawn|GetController _asbp_player)))
      (Default|PresentDialogueCamera _asbp_player_controller true (Math|Vector|Lerp(Vector) (Transformation|GetActorLocation _asbp_player) _returnvalue 0.5) _returnvalue))
    (:then_1
      (bind _returnvalue_2 (UserInterface|CreateWidget "/Game/Dialogue/UI/WBP_DialogueHUD.WBP_DialogueHUD_C"))
      (UserInterface|Viewport|AddtoViewport _returnvalue_2 0)
      (EventDispatchers|AssignOnClicked _returnvalue_2 (delegate Custom|OnClicked_Event))
      (Default|SetDialogue _returnvalue_2 _outspeakername (.OutItem (Utilities|Array|Random _outavailabledialogues))))))

(fn ConstructionScript)

(fn CanInteract
  (return true))