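; Player controller that routes Enhanced Input to the controlled pawn and manages a dialogue camera.
; Move is camera-relative and look drives controller yaw and pitch, while jump, attack and interact forward only to a BP_Player pawn.
; BeginPlay spawns a hidden BP_DialogueCamera and caches the original player.
; PresentDialogueCamera switches by possession rather than view target, placing the camera at a midpoint facing a look-at point or repossessing the player.
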(event Input|EnhancedActionEvents|EnhancedInputActionIA_Move
  (params (ActionValue :type Vector%202D%20Structure) (ElapsedSeconds :type Float%20%28double-precision%29) (TriggeredSeconds :type Float%20%28double-precision%29) (InputAction :type Input%20Action%20Object%20Reference :default "/Game/Input/Actions/IA_Move.IA_Move"))
  (bind _playercameramanager (Variables|Default|GetPlayerCameraManager))
  (bind _returnvalue (Camera|GetCameraRotation _playercameramanager))
  (Pawn|Input|AddMovementInput (Pawn|GetControlledPawn) (+ (* (.x ActionValue) (Math|Vector|GetRightVector _returnvalue)) (* (.y ActionValue) (Math|Vector|GetForwardVector _returnvalue))) 1.0 false))

(event Input|EnhancedActionEvents|EnhancedInputActionIA_Look
  (params (ActionValue :type Vector%202D%20Structure) (ElapsedSeconds :type Float%20%28double-precision%29) (TriggeredSeconds :type Float%20%28double-precision%29) (InputAction :type Input%20Action%20Object%20Reference :default "/Game/Input/Actions/IA_Look.IA_Look"))
  (bind _returnvalue (Pawn|GetControlledPawn))
  (Pawn|Input|AddControllerYawInput _returnvalue (.x ActionValue))
  (Pawn|Input|AddControllerPitchInput _returnvalue (.y ActionValue)))

(event Input|EnhancedActionEvents|EnhancedInputActionIA_Jump
  (params (ActionValue :type Boolean) (ElapsedSeconds :type Float%20%28double-precision%29) (TriggeredSeconds :type Float%20%28double-precision%29) (InputAction :type Input%20Action%20Object%20Reference :default "/Game/Input/Actions/IA_Jump.IA_Jump"))
  (bind _asbp_player (Utilities|Casting|CastToBP_Player (Pawn|GetControlledPawn)))
  (Character|Jump _asbp_player))

(event Input|EnhancedActionEvents|EnhancedInputActionIA_Attack
  (params (ActionValue :type Boolean) (ElapsedSeconds :type Float%20%28double-precision%29) (TriggeredSeconds :type Float%20%28double-precision%29) (InputAction :type Input%20Action%20Object%20Reference :default "/Game/Input/Actions/IA_Attack.IA_Attack"))
  (bind _asbp_player (Utilities|Casting|CastToBP_Player (Pawn|GetControlledPawn)))
  (Default|PerfomAttack _asbp_player))

(event Input|EnhancedActionEvents|EnhancedInputActionIA_Interact
  (params (ActionValue :type Boolean) (ElapsedSeconds :type Float%20%28double-precision%29) (TriggeredSeconds :type Float%20%28double-precision%29) (InputAction :type Input%20Action%20Object%20Reference :default "/Game/Input/Actions/IA_Interact.IA_Interact"))
  (bind _asbp_player (Utilities|Casting|CastToBP_Player (Pawn|GetControlledPawn)))
  (Default|Interact _asbp_player))

(event EventBeginPlay
  (Input|AddMappingContext (PlayerController|LocalPlayerSubsystems|GetEnhancedInputLocalPlayerSubsystem) "/Game/Input/IMC_Default.IMC_Default" 0 "(bIgnoreAllPressedKeysUntilRelease=True,bForceImmediately=False,bNotifyUserSettings=False)")
  (bind _returnvalue (Game|SpawnActorfromClass "/Game/Dialogue/BP_DialogueCamera.BP_DialogueCamera_C" (Math|Transform|MakeTransform "0, 0, 0") "Undefined" "MultiplyWithRoot" 0 0))
  (bind _output_get (Variables|Default|SetDialogueCamera _returnvalue))
  (Rendering|SetActorHiddenInGame _output_get true)
  (bind _asbp_player (Utilities|Casting|CastToBP_Player (Pawn|GetControlledPawn)))
  (Variables|Default|SetOrignalPlayer _asbp_player))

(fn ConstructionScript)

(fn PresentDialogueCamera
  (params (bShowDialogueCamera :type Boolean) (MidPoint :type Vector) (LookAtPoint :type Vector))
  (bind _dialoguecamera (Variables|Default|GetDialogueCamera))
  (bind _dialoguecamera_2 (Variables|Default|GetDialogueCamera))
  (Utilities|FlowControl|Sequence
    (:then_0
      (if bShowDialogueCamera
        (Pawn|Possess _dialoguecamera)
        (Rendering|SetActorHiddenInGame _dialoguecamera false)
        (else
          (Pawn|Possess (Variables|Default|GetOrignalPlayer))
          (Rendering|SetActorHiddenInGame _dialoguecamera true))))
    (:then_1
      (if bShowDialogueCamera
        (Transformation|SetActorLocation _dialoguecamera_2 MidPoint false true)
        (Transformation|SetActorRotation _dialoguecamera_2 (Math|Rotator|FindLookatRotation MidPoint LookAtPoint))))))