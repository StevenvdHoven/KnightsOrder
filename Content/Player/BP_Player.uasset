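; Player Blueprint with functions for attacking and interacting with objects in the world.
; PerfomAttack plays the axe-and-shield attack montage.
; Interact sphere-traces from the follow camera, with debug drawing, to its scaled forward vector, which is not offset by the camera location.
; A hit actor that casts to Interactable has its Interact called only if CanInteract allows it.
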(fn ConstructionScript
  (|CallParentFunction))

(fn PerfomAttack
  (Animation|PlayAnimMontage "/Game/FlexibleCombatSystem/Animations/OneHandShield/AxeAndShield_Attack_A_Montage.AxeAndShield_Attack_A_Montage" 1.0 "None"))

(fn Interact
  (bind _followcamera (Variables|Default|GetFollowCamera))
  (bind (_outhit _returnvalue) (Collision|SphereTraceForObjects (Transformation|GetWorldLocation _followcamera) (* (Math|Vector|GetForwardVector _followcamera) (Math|Float|MakeLiteralFloat 1e+04)) 5e+01 (Utilities|Array|MakeArray "ObjectTypeQuery1" "ObjectTypeQuery2" "ObjectTypeQuery3" "ObjectTypeQuery4") true (Utilities|Array|MakeArray self) "ForDuration"))
  (if _returnvalue
    (bind _asinteractable (Utilities|Casting|CastToInteractable (.HitActor (Collision|BreakHitResult _outhit))))
    (bind _binteractable (Default|CanInteract _asinteractable))
    (if _binteractable
      (Default|Interact _asinteractable))))